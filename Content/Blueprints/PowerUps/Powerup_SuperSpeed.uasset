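; Super speed power-up that temporarily doubles the walk speed of the player who activates it.
; On activation it stores that player and sets the Character Movement Component's MaxWalkSpeed to twice its current max speed.
; On expiry, if the stored player is still valid, it halves the current max speed rather than restoring a saved original value.
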(event `self.OnActivated`
  (params (ActiveFor :type "Actor Object Reference"))
  (bind _returnvalue (`self.GetComponentByClass` ActiveFor "/Script/Engine.CharacterMovementComponent"))
  (set `self.ActivatedForPlayer` ActiveFor)
  (set `CharacterMovementComponent.MaxWalkSpeed` (* (`MovementComponent.GetMaxSpeed` _returnvalue) 2.0) _returnvalue))

(event `self.OnExpired`
  (bind _activatedforplayer (`self.ActivatedForPlayer`))
  (bind _returnvalue (`self.GetComponentByClass` _activatedforplayer "/Script/Engine.CharacterMovementComponent"))
  (`/Engine/EditorBlueprintResources/StandardMacros.IsValid` _activatedforplayer
    (:`Is Valid`
      (set `CharacterMovementComponent.MaxWalkSpeed` (/ (`MovementComponent.GetMaxSpeed` _returnvalue) 2.0) _returnvalue))))

(fn `UserConstructionScript`)