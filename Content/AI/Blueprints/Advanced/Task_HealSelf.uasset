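; Behavior tree task that lets an AI-controlled pawn heal itself back to its default health.
; On execute, it finds the pawn's SHealthComponent and calls Heal with a per-tick amount, looping through a latent Delay while health stays below the default.
; It finishes successfully once health reaches the default, and calls Finish Abort when the pawn has no health component.
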(event `self.ReceiveExecuteAI`
  (params (OwnerController :type "AIController Object Reference") (ControlledPawn :type "Pawn Object Reference"))
  (bind _returnvalue (`Actor.GetComponentByClass` ControlledPawn "/Script/CoopShooter.SHealthComponent"))
  (`/Engine/EditorBlueprintResources/StandardMacros.IsValid` _returnvalue
    (:`Is Valid`
      (`SHealthComponent.Heal` _returnvalue (`self.HealPerTick`) :!label _label)
      (if (< (`SHealthComponent.Health` _returnvalue) (`SHealthComponent.DefaultHealth` _returnvalue))
        (`KismetSystemLibrary.Delay` (`self.HealITickInterval`))
        (goto _label)
        (else
          (`self.FinishExecute` true))))
    (:`Is Not Valid`
      (`self.FinishAbort`))))